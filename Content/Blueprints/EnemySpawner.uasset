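; EnemySpawner is a Blueprint that spawns AI enemies inside a box volume, up to a population cap.
; Its SpawnEnemy event counts every EnemyCharacter in the level and, if the count is below MaxEnemy, spawns one at a random point within SpawnVolume.
; Nothing in the file calls SpawnEnemy, since BeginPlay, overlap and Tick are empty disabled nodes.
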(event Custom|SpawnEnemy
  (bind _outactors (Actor|GetAllActorsOfClass "/Game/Blueprints/EnemyCharacter.EnemyCharacter_C"))
  (if (< (Utilities|Array|Length _outactors) (Variables|Default|GetMaxEnemy))
    (AI|SpawnAIFromClass "/Game/Blueprints/EnemyCharacter.EnemyCharacter_C" 0 (Math|Random|RandomPointinBoundingBox (Transformation|GetWorldLocation (Variables|Default|GetSpawnVolume)) (Components|Box|GetScaledBoxExtent (Variables|Default|GetSpawnVolume))) "0, 0, 0" false)))

(event EventBeginPlay)

(event Collision|EventActorBeginOverlap
  (params (OtherActor :type Actor%20Object%20Reference)))

(event EventTick
  (params (DeltaSeconds :type Float%20%28single-precision%29)))

(fn ConstructionScript)